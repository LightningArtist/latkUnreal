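; Brush stroke actor that rebuilds one drawn stroke from JSON data as a colored spline beam.
; On BeginPlay, after a zero-length delay, it converts each JSON point to a vector, swapping Y and Z and scaling up to Unreal space.
; It then adds a BP_SplineBeam child actor, feeds the points to its spline in world space and sets its color from the JSON.
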(event `self.ReceiveBeginPlay`
  (bind _strokejsondata (`self.StrokeJsonData`))
  (bind (_success _returnvalue) (`JsonFieldData.GetFloatArray` _strokejsondata "color"))
  (`KismetSystemLibrary.Delay` 0.0)
  (`KismetArrayLibrary.Array_Clear` (stale _output_get))
  (for _array_element (`.ReturnValue` (`JsonFieldData.GetObjectArray` _strokejsondata "points"))
    (bind _output_get (set `self.StrokePoints` (`self.StrokePoints`)))
    (bind (_success_2 _returnvalue_2) (`JsonFieldData.GetFloatArray` _array_element "co"))
    (bind _returnvalue_3 (* (`KismetMathLibrary.MakeVector` (`KismetArrayLibrary.Array_Get` _returnvalue_2) (`KismetArrayLibrary.Array_Get` _returnvalue_2 2) (`KismetArrayLibrary.Array_Get` _returnvalue_2 1)) 1000.0))
    (`KismetArrayLibrary.Array_Add` _output_get _returnvalue_3)
    (`KismetSystemLibrary.PrintString` (`KismetStringLibrary.BuildString_Vector` "" "co: " _returnvalue_3) false)
    (`KismetSystemLibrary.PrintString` (`KismetStringLibrary.BuildString_Int` "" "array: " (`KismetArrayLibrary.Array_Length` _output_get)) false))
  (bind _returnvalue_4 (`AddComponent|NODE_AddChildActorComponent-1`))
  (bind _asbp_spline_beam (cast `/Game/Blueprints/BP_SplineBeam` (`ChildActorComponent.ChildActor` _returnvalue_4)))
  (`SplineComponent.SetSplinePoints` (`/Game/Blueprints/BP_SplineBeam.MainSplinePath` _asbp_spline_beam) (`self.StrokePoints`) "World" true)
  (bind _output_get_2 (set `self.StrokeColor` (`KismetMathLibrary.MakeColor` (`KismetArrayLibrary.Array_Get` _returnvalue) (`KismetArrayLibrary.Array_Get` _returnvalue 1) (`KismetArrayLibrary.Array_Get` _returnvalue 2))))
  (set `/Game/Blueprints/BP_SplineBeam.Color` _output_get_2 _asbp_spline_beam))

(fn `UserConstructionScript`)