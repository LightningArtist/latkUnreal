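; Lightning Artist player actor that loads a layered grease pencil drawing from a Latk JSON file and plays it as a looping frame animation.
; On BeginPlay it spawns a BP_BrushLayer child actor for each layer and hands it that layer's JSON data.
; Tick accumulates time against the frame rate, then advances every layer's current frame, wrapping each at its own length.
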(event `self.ReceiveBeginPlay`
  (bind _output_get (set `self.MainJsonData` (`JsonFieldData.Create`)))
  (bind _returnvalue (`JsonFieldData.FromFile` _output_get "Latk/layer_test.json"))
  (`KismetSystemLibrary.PrintString` (`KismetStringLibrary.BuildString_Bool` "" "*** read file: " _returnvalue))
  (for _array_element (`.ReturnValue` (`JsonFieldData.GetObjectArray` _output_get "grease_pencil"))
    (for _array_element_2 (`.ReturnValue` (`JsonFieldData.GetObjectArray` _array_element "layers"))
      (bind _returnvalue_2 (`AddComponent|NODE_AddChildActorComponent-13`))
      (bind _asbp_brush_layer (cast `/Game/Blueprints/BP_BrushLayer` (`ChildActorComponent.ChildActor` _returnvalue_2)))
      (set `/Game/Blueprints/BP_BrushLayer.LayerJsonData` _array_element_2 _asbp_brush_layer))))

(event `self.ReceiveTick`
  (params (DeltaSeconds :type "Float (single-precision)"))
  (bind _intervaltime (`self.IntervalTime`))
  (`/Engine/EditorBlueprintResources/StandardMacros.CompareFloat` _intervaltime (/ 1.0 (`self.FrameRate`))
    (:`>`
      (set `self.IntervalTime` 0.0 :!label _label)
      (for _array_element (`self.GetAllChildActors` false)
        (bind _asbp_brush_layer (cast `/Game/Blueprints/BP_BrushLayer` _array_element))
        (bind _returnvalue (+ (`/Game/Blueprints/BP_BrushLayer.LayerFrameCurrent` _asbp_brush_layer) 1))
        (`/Engine/EditorBlueprintResources/StandardMacros.CompareInt` _returnvalue (- (`/Game/Blueprints/BP_BrushLayer.LayerLength` _asbp_brush_layer) 1)
          (:`>`
            (set `/Game/Blueprints/BP_BrushLayer.LayerFrameCurrent` 0 _asbp_brush_layer))
          (:`==`
            (set `/Game/Blueprints/BP_BrushLayer.LayerFrameCurrent` _returnvalue _asbp_brush_layer :!label _label_2))
          (:`<`
            (goto _label_2)))))
    (:`==`
      (goto _label))
    (:`<`
      (set `self.IntervalTime` (+ _intervaltime DeltaSeconds)))))

(fn `UserConstructionScript`)