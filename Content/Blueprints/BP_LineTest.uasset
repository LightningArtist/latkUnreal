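; Test actor that loads a Latk grease pencil drawing from a local JSON file and rebuilds it as colored spline beams on BeginPlay.
; Nested loops walk layers, frames, strokes and points, swapping Y and Z and scaling up the coordinates.
; Each stroke spawns a BP_SplineBeam child actor with world-space points and stroke color, so all frames appear at once.
; An HTTP download of the same file is left unconnected.
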(event `self.ReceiveBeginPlay`
  (bind _output_get (set `self.JsonData` (`JsonFieldData.Create`)))
  (bind _returnvalue (`JsonFieldData.FromFile` _output_get "Latk/layer_test.json"))
  (`KismetSystemLibrary.PrintString` (`KismetStringLibrary.BuildString_Bool` "" "*** read file: " _returnvalue))
  (for _array_element (`.ReturnValue` (`JsonFieldData.GetObjectArray` _output_get "grease_pencil"))
    (for _array_element_2 (`.ReturnValue` (`JsonFieldData.GetObjectArray` _array_element "layers"))
      (for _array_element_3 (`.ReturnValue` (`JsonFieldData.GetObjectArray` _array_element_2 "frames"))
        (for _array_element_4 (`.ReturnValue` (`JsonFieldData.GetObjectArray` _array_element_3 "strokes"))
          (`KismetArrayLibrary.Array_Clear` (stale _output_get_2))
          (for _array_element_5 (`.ReturnValue` (`JsonFieldData.GetObjectArray` _array_element_4 "points"))
            (bind _output_get_2 (set `self.PointsArray` (`self.PointsArray`)))
            (bind (_success _returnvalue_2) (`JsonFieldData.GetFloatArray` _array_element_5 "co"))
            (bind _returnvalue_3 (* (`KismetMathLibrary.MakeVector` (`KismetArrayLibrary.Array_Get` _returnvalue_2) (`KismetArrayLibrary.Array_Get` _returnvalue_2 2) (`KismetArrayLibrary.Array_Get` _returnvalue_2 1)) 1000.0))
            (`KismetArrayLibrary.Array_Add` _output_get_2 _returnvalue_3)
            (`KismetSystemLibrary.PrintString` (`KismetStringLibrary.BuildString_Vector` "" "co: " _returnvalue_3) false)
            (`KismetSystemLibrary.PrintString` (`KismetStringLibrary.BuildString_Int` "" "array: " (`KismetArrayLibrary.Array_Length` _output_get_2)) false))
          (bind _returnvalue_4 (`AddComponent|NODE_AddChildActorComponent-6`))
          (bind _asbp_spline_beam (cast `/Game/Blueprints/BP_SplineBeam` (`ChildActorComponent.ChildActor` _returnvalue_4)))
          (`SplineComponent.SetSplinePoints` (`/Game/Blueprints/BP_SplineBeam.MainSplinePath` _asbp_spline_beam) (`self.PointsArray`) "World" true)
          (bind (_success_2 _returnvalue_5) (`JsonFieldData.GetFloatArray` _array_element_4 "color"))
          (set `/Game/Blueprints/BP_SplineBeam.Color` (`KismetMathLibrary.MakeColor` (`KismetArrayLibrary.Array_Get` _returnvalue_5) (`KismetArrayLibrary.Array_Get` _returnvalue_5 1) (`KismetArrayLibrary.Array_Get` _returnvalue_5 2)) _asbp_spline_beam))))))

(event `OnGetResult_Event_0`
  (params (bSuccess :type Boolean) (JSON :type "JsonFieldData Object Reference") (Status :type "EJSONResult Enum")))

(fn `UserConstructionScript`)