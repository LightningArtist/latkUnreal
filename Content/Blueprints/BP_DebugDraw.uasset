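; BP_DebugDraw renders a stroke in a Lightning Artist drawing by tracing its spline with debug lines.
; On BeginPlay it caches the scene's BP_LightningArtist for global thickness and frame rate.
; Each Tick, if its grandparent BP_BrushFrame is visible, it draws straight segments between consecutive MainSplinePath points, each lasting one animation frame.
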(event `self.ReceiveTick`
  (params (DeltaSeconds :type "Float (single-precision)"))
  (bind _mainsplinepath (`self.MainSplinePath`))
  (bind _asbp_brush_frame (cast `/Game/Blueprints/BP_BrushFrame` (`self.GetParentActor` (`self.GetParentActor`))))
  (if (`/Game/Blueprints/BP_BrushFrame.FrameVisible` _asbp_brush_frame)
    (for _index (range (+ (- (`SplineComponent.GetNumberOfSplinePoints` _mainsplinepath) 2) 1))
      (`KismetSystemLibrary.DrawDebugLine` (`SplineComponent.GetLocationAtSplinePoint` _mainsplinepath _index "World") (`SplineComponent.GetLocationAtSplinePoint` _mainsplinepath (+ _index 1) "World") (`self.Color`) (/ 1.0 (`/Game/Blueprints/BP_LightningArtist.FrameRate` (stale `self.ReceiveBeginPlay` _asbp_lightning_artist))) (`/Game/Blueprints/BP_LightningArtist.GlobalThickness` (stale `self.ReceiveBeginPlay` _asbp_lightning_artist))))))

(event `self.ReceiveBeginPlay`
  (`KismetSystemLibrary.Delay` 0.0)
  (bind _outactors (`GameplayStatics.GetAllActorsOfClass` "/Game/Blueprints/BP_LightningArtist.BP_LightningArtist_C"))
  (bind _asbp_lightning_artist (cast `/Game/Blueprints/BP_LightningArtist` (`KismetArrayLibrary.Array_Get` _outactors))))

(fn `UserConstructionScript`)