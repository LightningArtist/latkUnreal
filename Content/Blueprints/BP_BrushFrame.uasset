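; BP_BrushFrame is one frame of a brush-stroke drawing, built from JSON and shown or hidden as a whole.
; After a zero-length delay on BeginPlay, it adds a child BP_BrushStroke per "strokes" entry, passing each its JSON.
; On Tick, whenever BP_LightningArtist's IntervalTime equals zero, it applies FrameVisible to a scene component on each stroke's first child actor, propagating to children.
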(event `self.ReceiveBeginPlay`
  (`KismetSystemLibrary.Delay` 0.0)
  (for (_array_element _array_index) (`.ReturnValue` (`JsonFieldData.GetObjectArray` (`self.FrameJsonData`) "strokes"))
    (bind _returnvalue (`AddComponent|NODE_AddChildActorComponent-3`))
    (bind _asbp_brush_stroke (cast `/Game/Blueprints/BP_BrushStroke` (`ChildActorComponent.ChildActor` _returnvalue)))
    (set `/Game/Blueprints/BP_BrushStroke.StrokeJsonData` _array_element _asbp_brush_stroke))
  (set `self.FrameStrokeCount` _array_index)
  (set `self.FrameReady` true)
  (bind _outactors (`GameplayStatics.GetAllActorsOfClass` "/Game/Blueprints/BP_LightningArtist.BP_LightningArtist_C")))

(event `self.ReceiveTick`
  (params (DeltaSeconds :type "Float (single-precision)"))
  (if (`self.FrameReady`)
    (`/Engine/EditorBlueprintResources/StandardMacros.CompareFloat` (`/Game/Blueprints/BP_LightningArtist.IntervalTime` (`KismetArrayLibrary.Array_Get` (stale `self.ReceiveBeginPlay` _outactors)))
      (:`==`
        (for _array_element (`self.GetAllChildActors` false)
          (`SceneComponent.SetVisibility` (`self.GetComponentByClass` (`KismetArrayLibrary.Array_Get` (`self.GetAllChildActors` _array_element false)) "/Script/Engine.SceneComponent") (`self.FrameVisible`) true))))))

(fn `UserConstructionScript`)