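; BP_SplineBeam draws a colored particle beam along its MainSplinePath spline.
; One tick after BeginPlay, it spawns a P_Beam emitter per spline segment, each tinted through a dynamic M_Beam2 material using Color.
; Each segment's endpoint locations and tangents feed the beam's source and target parameters, so it follows the curve.
; Rebuild reruns the same spawning without removing existing emitters.
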(event `self.ReceiveBeginPlay`
  (bind _mainsplinepath (`self.MainSplinePath`))
  (`KismetSystemLibrary.Delay` 0.0 :!label _label)
  (for _index (range (+ (- (`SplineComponent.GetNumberOfSplinePoints` _mainsplinepath) 2) 1))
    (bind _returnvalue (`SplineComponent.GetLocationAtSplinePoint` _mainsplinepath _index "World"))
    (bind _returnvalue_2 (`GameplayStatics.SpawnEmitterAttached` "/Game/Particles/P_Beam.P_Beam" _mainsplinepath "None" _returnvalue))
    (bind _returnvalue_3 (`PrimitiveComponent.CreateDynamicMaterialInstance` _returnvalue_2 0 "/Game/Materials/M_Beam2.M_Beam2"))
    (`MaterialInstanceDynamic.SetVectorParameterValue` _returnvalue_3 "MainColor" (`self.Color`))
    (`ParticleSystemComponent.SetVectorParameter` _returnvalue_2 "Source" _returnvalue)
    (`ParticleSystemComponent.SetVectorParameter` _returnvalue_2 "Source_Tan" (`SplineComponent.GetTangentAtDistanceAlongSpline` _mainsplinepath (`SplineComponent.GetDistanceAlongSplineAtSplinePoint` _mainsplinepath _index) "World"))
    (`ParticleSystemComponent.SetVectorParameter` _returnvalue_2 "Target" (`SplineComponent.GetLocationAtSplinePoint` _mainsplinepath (+ _index 1) "World"))
    (`ParticleSystemComponent.SetVectorParameter` _returnvalue_2 "Target_Tan" (`SplineComponent.GetTangentAtDistanceAlongSpline` _mainsplinepath (`SplineComponent.GetDistanceAlongSplineAtSplinePoint` _mainsplinepath (+ _index 1)) "World"))))

(event `Rebuild`
  (goto _label))

(fn `UserConstructionScript`)